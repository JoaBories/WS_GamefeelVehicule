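; GM_Tank, likely the tank game mode by its name, provides a Pause event that toggles the game's paused state and pause menu.
; Pausing creates a fresh WBP_PauseMenu, stores it and adds it to the viewport, without changing input mode or cursor here.
; Unpausing restores game-only input, hides the mouse cursor, then deactivates and removes the stored menu.
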(event `Pause`
  (bind _returnvalue (`GameplayStatics.GetPlayerController` 0))
  (bind _pausemenu (`self.PauseMenu`))
  (if (`GameplayStatics.IsGamePaused`)
    (`GameplayStatics.SetGamePaused` false)
    (`WidgetBlueprintLibrary.SetInputMode_GameOnly` _returnvalue)
    (set `PlayerController.bShowMouseCursor` false _returnvalue)
    (`CommonActivatableWidget.DeactivateWidget` _pausemenu)
    (`Widget.RemoveFromParent` _pausemenu)
    (else
      (`GameplayStatics.SetGamePaused` true)
      (bind _returnvalue_2 (`|CreateWidget` "/Game/01_BP/03_Ui/WBP_PauseMenu.WBP_PauseMenu_C"))
      (bind _output_get (set `self.PauseMenu` _returnvalue_2))
      (`UserWidget.AddToViewport` _output_get 0))))

(fn `UserConstructionScript`)