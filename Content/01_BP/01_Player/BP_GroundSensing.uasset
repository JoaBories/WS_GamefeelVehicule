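; BP_GroundSensing is a component that detects the ground beneath its position on the owning actor.
; Each Tick it line traces straight down along world Z by TraceDistance on the Visibility channel, ignoring the owner and drawing debug for one frame.
; A hit updates OnGround, HitLocation and HitNormal, while a miss clears only OnGround, leaving the last location and normal in place.
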(event `self.ReceiveTick`
  (params (DeltaSeconds :type "Float (single-precision)"))
  (bind _returnvalue (`self.K2_GetComponentLocation`))
  (bind (_outhit _returnvalue_2) (`KismetSystemLibrary.LineTraceSingle` _returnvalue (- _returnvalue (* (`KismetMathLibrary.GetUpVector` (struct)) (`self.TraceDistance`))) "TraceTypeQuery1" false (`|MakeArray` (`self.GetOwner`)) "ForOneFrame"))
  (if _returnvalue_2
    (bind (_bblockinghit _binitialoverlap _time _distance _location _impactpoint _normal) (`GameplayStatics.BreakHitResult` _outhit))
    (set `self.bOnGround` _bblockinghit)
    (set `self.HitLocation` _location)
    (set `self.HitNormal` _normal)
    (else
      (set `self.bOnGround` false))))