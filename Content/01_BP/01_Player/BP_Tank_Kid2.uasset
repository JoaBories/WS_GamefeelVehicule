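; BP_Tank_Kid2 is a child tank Blueprint that caches its BP_GroundSensing components at BeginPlay and otherwise defers to its parent.
; A disconnected, never-run graph averages ground normals and heights across those sensors, dividing by the grounded count.
; That unused logic would tilt the Tank to the averaged normal, correct its height and move it forward at an interpolated speed.
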(event `self.ReceiveBeginPlay`
  (`parent.ReceiveBeginPlay`)
  (set `self.GroundSensingArray` (`self.K2_GetComponentsByClass` "/Game/01_BP/01_Player/BP_GroundSensing.BP_GroundSensing_C")))

(event `self.ReceiveTick`
  (params (DeltaSeconds :type "Float (single-precision)"))
  (`parent.ReceiveTick` DeltaSeconds))

(fn `UserConstructionScript`
  (`parent.UserConstructionScript`))