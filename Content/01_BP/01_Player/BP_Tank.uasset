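; Player tank pawn with independently rotating base and turret, pitching cannon, rate-limited shooting, rechargeable nitro boost and damageable life.
; Input and Tick write FloatingPawnMovement velocity directly, adding throttle, gravity and separate side and forward friction, tuned through DaMovements.
; Shots spawn BP_TankProjectile aimed at a camera sphere-trace hit, falling back to muzzle rotation.
; BeginPlay creates the HUD, debug drawing runs every tick, and ground-alignment code is left disconnected.
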(event `EnhancedInput|/Game/01_BP/00_Inputs/InputActions/IA_Nitro`
  (params (ActionValue :type Boolean) (ElapsedSeconds :type "Float (double-precision)") (TriggeredSeconds :type "Float (double-precision)") (InputAction :type "InputAction Object Reference" :default "/Game/01_BP/00_Inputs/InputActions/IA_Nitro.IA_Nitro"))
  (bind _damovements (`self.DaMovements`))
  (:`Started`
    (set `self.Nitroing` true)
    (set `self.RechargingNitro` false)
    (`ActorComponent.Activate` (`self.NitroNiagara`) false))
  (:`Completed`
    (set `self.Nitroing` false)
    (`ActorComponent.Deactivate` (`self.NitroNiagara`))
    (if (not (>= (`self.Nitro`) (`/Game/01_BP/04_DataAssets/BP_DA_TankMovements.NitroSlowRechargeTreshold` _damovements)))
      (`KismetSystemLibrary.RetriggerableDelay` (`/Game/01_BP/04_DataAssets/BP_DA_TankMovements.NitroSlowRechargeDelay` _damovements)))
    (set `self.RechargingNitro` true)))

(event `self.ReceiveBeginPlay`
  (bind _damovements (`self.DaMovements`))
  (bind _returnvalue (`|CreateWidget` "/Game/01_BP/03_Ui/WBP_HUD.WBP_HUD_C"))
  (`UserWidget.AddToViewport` _returnvalue 0)
  (set `self.Life` (`/Game/01_BP/04_DataAssets/BP_DA_TankMovements.MaxLife` _damovements))
  (set `self.Nitro` (`/Game/01_BP/04_DataAssets/BP_DA_TankMovements.NitroMax` _damovements)))

(event `EnhancedInput|/Game/01_BP/00_Inputs/InputActions/IA_ResetTurret`
  (params (ActionValue :type Boolean) (ElapsedSeconds :type "Float (double-precision)") (TriggeredSeconds :type "Float (double-precision)") (InputAction :type "InputAction Object Reference" :default "/Game/01_BP/00_Inputs/InputActions/IA_ResetTurret.IA_ResetTurret"))
  (:`Triggered`
    (set `self.ResetingTurret` true)))

(event `EnhancedInput|/Game/01_BP/00_Inputs/InputActions/IA_Shoot`
  (params (ActionValue :type Boolean) (ElapsedSeconds :type "Float (double-precision)") (TriggeredSeconds :type "Float (double-precision)") (InputAction :type "InputAction Object Reference" :default "/Game/01_BP/00_Inputs/InputActions/IA_Shoot.IA_Shoot"))
  (:`Triggered`
    (if (`self.CanShoot`)
      (`self.Shoot`)
      (set `self.CanShoot` false)
      (set `self.Shooting` true)
      (`KismetSystemLibrary.Delay` (/ 1.0 (`/Game/01_BP/04_DataAssets/BP_DA_TankMovements.ShootRate` (`self.DaMovements`))))
      (set `self.CanShoot` true)
      (set `self.Shooting` false))))

(event `EnhancedInput|/Game/01_BP/00_Inputs/InputActions/IA_RotateTurret`
  (params (ActionValue :type "Vector2D Structure") (ElapsedSeconds :type "Float (double-precision)") (TriggeredSeconds :type "Float (double-precision)") (InputAction :type "InputAction Object Reference" :default "/Game/01_BP/00_Inputs/InputActions/IA_RotateTurret.IA_RotateTurret"))
  (bind (_x _y) (`KismetMathLibrary.BreakVector2D` ActionValue))
  (:`Triggered`
    (if (not (`self.ResetingTurret`))
      (`self.RotateTurret` _x)
      (`self.RotateCanon` _y))))

(event `EnhancedInput|/Game/01_BP/00_Inputs/InputActions/IA_Throttle`
  (params (ActionValue :type "Float (double-precision)") (ElapsedSeconds :type "Float (double-precision)") (TriggeredSeconds :type "Float (double-precision)") (InputAction :type "InputAction Object Reference" :default "/Game/01_BP/00_Inputs/InputActions/IA_Throttle.IA_Throttle"))
  (:`Triggered`
    (bind _output_get (set `self.Acceleration` (* (`SceneComponent.GetForwardVector` (`self.TankBase`)) ActionValue (`/Game/01_BP/04_DataAssets/BP_DA_TankMovements.GetAcceleration` (`self.DaMovements`) (`self.HasNitro`) (> ActionValue 0.0)))))
    (bind _output_get_2 (set `MovementComponent.Velocity` (+ (`MovementComponent.Velocity` (`self.FloatingPawnMovement`)) (* _output_get (`GameplayStatics.GetWorldDeltaSeconds`))) (`self.FloatingPawnMovement`)))
    (set `self.Accelerating` (> (`KismetMathLibrary.Dot_VectorVector` (`self.Acceleration`) _output_get_2) 0.0)))
  (:`Completed`
    (set `self.Accelerating` false)))

(event `EnhancedInput|/Game/01_BP/00_Inputs/InputActions/IA_RotateBase`
  (params (ActionValue :type "Float (double-precision)") (ElapsedSeconds :type "Float (double-precision)") (TriggeredSeconds :type "Float (double-precision)") (InputAction :type "InputAction Object Reference" :default "/Game/01_BP/00_Inputs/InputActions/IA_RotateBase.IA_RotateBase"))
  (bind _returnvalue (`self.GetRotationForBase` ActionValue))
  (:`Triggered`
    (`SceneComponent.K2_AddLocalRotation` (`self.TankBase`) (`KismetMathLibrary.MakeRotator` 0.0 0.0 _returnvalue) false false)
    (`SceneComponent.K2_AddLocalRotation` (`self.TankTurret`) (`KismetMathLibrary.MakeRotator` 0.0 0.0 (* _returnvalue -1.0)) false false)))

(event `self.ReceiveTick`
  (params (DeltaSeconds :type "Float (single-precision)"))
  (`self.ApplyFrictions` DeltaSeconds)
  (`self.ResetTurret`)
  (`self.Debug`)
  (bind _output_get (set `MovementComponent.Velocity` (+ (`MovementComponent.Velocity` (`self.FloatingPawnMovement`)) (`KismetMathLibrary.MakeVector` 0.0 0.0 (* (`/Game/01_BP/04_DataAssets/BP_DA_TankMovements.GravityForce` (`self.DaMovements`)) DeltaSeconds -100.0))) (`self.FloatingPawnMovement`)))
  (`self.UpdateNitro` DeltaSeconds)
  (`NiagaraComponent.SetVariableFloat` (`self.NitroNiagara`) "Length" (* (`KismetMathLibrary.VSize` _output_get) 0.1)))

(event `Debug`
  (bind _returnvalue (`self.K2_GetActorLocation`))
  (bind _returnvalue_2 (`self.K2_GetActorLocation`))
  (`KismetSystemLibrary.DrawDebugArrow` _returnvalue_2 (+ _returnvalue_2 (* (`MovementComponent.Velocity` (`self.FloatingPawnMovement`)) 1.0)) 5.0 (struct :`R` 1.0 :`G` 0.831964 :`A` 1.0) 0.0 1.0)
  (`KismetSystemLibrary.PrintString` (`KismetStringLibrary.Conv_VectorToString` (`MovementComponent.Velocity` (`self.FloatingPawnMovement`))) true false (struct :`R` 1.0 :`G` 0.885596 :`A` 1.0) 0.0)
  (`KismetSystemLibrary.PrintString` (`KismetStringLibrary.Concat_StrStr` "Pv : " (`KismetStringLibrary.Conv_DoubleToString` (`self.Life`))) true false (struct :`R` 0.01237 :`G` 0.791667 :`B` 0.201685 :`A` 1.0) 0.0)
  (`KismetSystemLibrary.PrintString` (`KismetStringLibrary.Concat_StrStr` "Nitro : " (`KismetStringLibrary.Conv_DoubleToString` (`self.Nitro`))) true false (struct :`R` 0.003575 :`G` 0.636292 :`B` 0.791667 :`A` 1.0) 0.0)
  (`KismetSystemLibrary.DrawDebugArrow` _returnvalue (+ _returnvalue (* (`self.Acceleration`) 1.0)) 5.0 (struct :`R` 1.0 :`G` 0.186049 :`B` 0.786379 :`A` 1.0) 0.0 1.0))

(event `self.ReceiveAnyDamage`
  (params (Damage :type "Float (single-precision)") (DamageType :type "DamageType Object Reference") (InstigatedBy :type "Controller Object Reference") (DamageCauser :type "Actor Object Reference"))
  (set `self.Life` (`KismetMathLibrary.FClamp` (- (`self.Life`) Damage) 0.0 (`/Game/01_BP/04_DataAssets/BP_DA_TankMovements.MaxLife` (`self.DaMovements`)))))

(fn `ApplyFrictions`
  (params (DeltaTime :type "Float (single-precision)"))
  (locals (ForwardVelocity :type "Float (double-precision)" :default 0.0) (SideVelocity :type "Float (double-precision)" :default 0.0))
  (bind _maxvelocity (`/Game/01_BP/04_DataAssets/BP_DA_TankMovements.GetMaxVelocity` (`self.DaMovements`) (`self.HasNitro`) (`self.IsGoingForward`)))
  (bind _returnvalue (`KismetMathLibrary.Abs` (`local.ForwardVelocity`)))
  (bind (_velocity_x _velocity_y _velocity_z) (`KismetMathLibrary.BreakVector` (`MovementComponent.Velocity` (`self.FloatingPawnMovement`))))
  (bind _friction (`/Game/01_BP/04_DataAssets/BP_DA_TankMovements.Friction` (`self.DaMovements`)))
  (bind _returnvalue_2 (`KismetMathLibrary.Conv_VectorToVector2D` (`MovementComponent.Velocity` (`self.FloatingPawnMovement`))))
  (set `local.ForwardVelocity` (`KismetMathLibrary.DotProduct2D` _returnvalue_2 (`KismetMathLibrary.Normal2D` (`KismetMathLibrary.Conv_VectorToVector2D` (`SceneComponent.GetForwardVector` (`self.TankBase`))))))
  (set `local.SideVelocity` (`KismetMathLibrary.DotProduct2D` _returnvalue_2 (`KismetMathLibrary.Normal2D` (`KismetMathLibrary.Conv_VectorToVector2D` (`SceneComponent.GetRightVector` (`self.TankBase`))))))
  (bind _output_get (set `MovementComponent.Velocity` (+ (* (+ (* (`KismetMathLibrary.Vector_Normal2D` (`SceneComponent.GetRightVector` (`self.TankBase`))) (`/Game/01_BP/BPFL_KiliLibrary.KL_1-x` (* (`local.DeltaTime`) (`/Game/01_BP/04_DataAssets/BP_DA_TankMovements.SideFriction` (`self.DaMovements`)))) (`local.SideVelocity`)) (* (`KismetMathLibrary.Vector_Normal2D` (`SceneComponent.GetForwardVector` (`self.TankBase`))) (`local.ForwardVelocity`))) (`/Game/01_BP/BPFL_KiliLibrary.KL_1-x` (* (`KismetMathLibrary.SelectFloat` (`KismetMathLibrary.SelectFloat` 0.0 _friction (`self.Accelerating`)) (* _friction (/ _returnvalue _maxvelocity) (`/Game/01_BP/04_DataAssets/BP_DA_TankMovements.MaxVelocityMult` (`self.DaMovements`))) (> _maxvelocity _returnvalue)) (`local.DeltaTime`)))) (`KismetMathLibrary.MakeVector` 0.0 0.0 _velocity_z)) (`self.FloatingPawnMovement`)))
  (if (<= (`KismetMathLibrary.VSizeXY` _output_get) (`self.ZeroVelocityTreshold`))
    (set `MovementComponent.Velocity` (`KismetMathLibrary.MakeVector` 0.0 0.0 (.z _output_get)) (`self.FloatingPawnMovement`))))

(fn `CheckGround`
  (params (CheckPos :type "SceneComponent Object Reference"))
  (returns (Distance :type "Float (single-precision)") (Normal :type "Vector Structure"))
  (bind (_start _end) (`/Game/01_BP/BPFL_KiliLibrary.KL_GetLinetraceGoal` (`SceneComponent.K2_GetComponentLocation` CheckPos) (`KismetMathLibrary.NegateVector` (`SceneComponent.GetUpVector` CheckPos)) 0.0 (`self.CheckGroundMaxDistance`)))
  (bind _outhit (`KismetSystemLibrary.LineTraceSingle` :`Start` _start :`End` _end :`TraceChannel` "TraceTypeQuery1" :`DrawDebugType` "ForOneFrame"))
  (bind (_bblockinghit _binitialoverlap _time _distance _location _impactpoint _normal) (`GameplayStatics.BreakHitResult` _outhit))
  (return _distance _normal))

(fn `CheckGrounds`
  (returns (Up :type "Vector Structure"))
  (locals (TtNormals :type "Vector Structure" :default (0.0 0.0 0.0)) (TtDistance :type "Float (double-precision)"))
  (bind _distance (`self.CheckGround` null))
  (bind _distance_2 (`self.CheckGround` null))
  (bind _returnvalue (/ (- _distance _distance_2) (`self.CheckGroundMaxDistance`)))
  (`KismetSystemLibrary.PrintString` (`KismetStringLibrary.Conv_DoubleToString` _returnvalue) true true (struct :`G` 0.66 :`B` 1.0 :`A` 1.0) 0.0)
  (`KismetSystemLibrary.PrintString` (`KismetStringLibrary.Conv_DoubleToString` 0.0) true true (struct :`R` 1.0 :`G` 0.05036 :`A` 1.0) 0.0)
  (return (`KismetMathLibrary.Normal` (`KismetMathLibrary.SelectVector` (`KismetMathLibrary.VLerp` (`KismetMathLibrary.Normal` (`KismetMathLibrary.Conv_Vector2DToVector` (`KismetMathLibrary.Conv_VectorToVector2D` (- (0.0 0.0 0.0) (`self.K2_GetActorLocation`))))) (0.0 0.0 1.0) (`KismetMathLibrary.FClamp` (+ _returnvalue 1.0))) (`KismetMathLibrary.VLerp` (0.0 0.0 1.0) (`KismetMathLibrary.Normal` (`KismetMathLibrary.Conv_Vector2DToVector` (`KismetMathLibrary.Conv_VectorToVector2D` (- (0.0 0.0 0.0) (`self.K2_GetActorLocation`))))) (`KismetMathLibrary.FClamp` _returnvalue)) (< _returnvalue 0.0)))))

(fn `GetRotationForBase`
  (params (Input :type "Float (double-precision)"))
  (returns (ReturnValue :type "Float (double-precision)"))
  (bind _returnvalue (`KismetMathLibrary.DotProduct2D` (`KismetMathLibrary.Normal2D` (`KismetMathLibrary.Conv_VectorToVector2D` (`SceneComponent.GetForwardVector` (`self.TankBase`)))) (`KismetMathLibrary.Conv_VectorToVector2D` (`MovementComponent.Velocity` (`self.FloatingPawnMovement`)))))
  (return (* (`local.Input`) (`GameplayStatics.GetWorldDeltaSeconds`) (`/Game/01_BP/04_DataAssets/BP_DA_TankMovements.GetRotateSpeed` (`self.DaMovements`) (`self.HasNitro`)) (`KismetMathLibrary.SelectFloat` 1.0 (`KismetMathLibrary.SignOfFloat` _returnvalue) (<= (`KismetMathLibrary.Abs` _returnvalue) (`self.ZeroVelocityTreshold`))))))

(fn `HasNitro`
  (returns (Nitroing :type Boolean))
  (return (and (`self.Nitroing`) (> (`self.Nitro`) 0.0))))

(fn `IsGoingForward`
  (returns (Forward :type Boolean) (Dot :type "Float (double-precision)"))
  (bind _returnvalue (`KismetMathLibrary.Dot_VectorVector` (`KismetMathLibrary.Vector_Normal2D` (`SceneComponent.GetForwardVector` (`self.TankBase`))) (`KismetMathLibrary.Vector_Normal2D` (`MovementComponent.Velocity` (`self.FloatingPawnMovement`)))))
  (return (> _returnvalue 0.0) _returnvalue))

(fn `ResetTurret`
  (bind _relativerotation (`SceneComponent.RelativeRotation` (`self.TankTurret`)))
  (if (`self.ResetingTurret`)
    (if (== _relativerotation (struct) :`ErrorTolerance` 1.0)
      (set `self.ResetingTurret` false)
      (else
        (`SceneComponent.K2_SetRelativeRotation` (`self.TankTurret`) (`KismetMathLibrary.RLerp` _relativerotation (struct) 0.1 true) false false)))))

(fn `RotateCanon`
  (params (InputY :type "Float (double-precision)"))
  (bind (_relativerotation_roll _relativerotation_pitch _relativerotation_yaw) (`KismetMathLibrary.BreakRotator` (`SceneComponent.RelativeRotation` (`self.SpringArm`))))
  (bind _outpitch (`/Game/01_BP/04_DataAssets/BP_DA_TankMovements.ClampCanonPitch` (`self.DaMovements`) (+ (.pitch (`SceneComponent.RelativeRotation` (`self.TankCanon`))) (* (`/Game/01_BP/04_DataAssets/BP_DA_TankMovements.CanonPitchSpeed` (`self.DaMovements`)) InputY (`GameplayStatics.GetWorldDeltaSeconds`)))))
  (`SceneComponent.K2_SetRelativeRotation` (`self.TankCanon`) (`KismetMathLibrary.MakeRotator` 0.0 _outpitch) false false)
  (`SceneComponent.K2_SetRelativeRotation` (`self.SpringArm`) (`KismetMathLibrary.MakeRotator` 0.0 _outpitch _relativerotation_yaw) false false))

(fn `RotateTurret`
  (params (InputX :type "Float (double-precision)"))
  (`SceneComponent.K2_AddLocalRotation` (`self.TankTurret`) (`KismetMathLibrary.MakeRotator` 0.0 0.0 (* (`/Game/01_BP/04_DataAssets/BP_DA_TankMovements.TurretRotateSpeed` (`self.DaMovements`)) (`GameplayStatics.GetWorldDeltaSeconds`) InputX)) false false))

(fn `Shoot`
  (bind _camera (`self.Camera`))
  (bind _projectilespawn (`self.ProjectileSpawn`))
  (bind _returnvalue (`SceneComponent.K2_GetComponentLocation` _projectilespawn))
  (bind (_start _end) (`/Game/01_BP/BPFL_KiliLibrary.KL_GetLinetraceGoal` (`SceneComponent.K2_GetComponentLocation` _camera) (`SceneComponent.GetForwardVector` _camera) 0.0 10000.0))
  (bind _outhit (`KismetSystemLibrary.SphereTraceSingleForObjects` :`Start` _start :`End` _end :`Radius` (`/Game/01_BP/04_DataAssets/BP_DA_TankMovements.ShootRadius` (`self.DaMovements`)) :`ObjectTypes` (`|MakeArray` "ObjectTypeQuery1" "ObjectTypeQuery2" :!type "EObjectTypeQuery Enum") :`DrawTime` 0.5))
  (bind (_bblockinghit _binitialoverlap _time _distance _location) (`GameplayStatics.BreakHitResult` _outhit))
  (`|SpawnActorFromClass` "/Game/01_BP/01_Player/BP_TankProjectile.BP_TankProjectile_C" (`KismetMathLibrary.MakeTransform` _returnvalue (`KismetMathLibrary.SelectRotator` (`KismetMathLibrary.MakeRotFromX` (`KismetMathLibrary.Normal` (- _location _returnvalue))) (`SceneComponent.K2_GetComponentRotation` _projectilespawn) _bblockinghit)) "AlwaysSpawn" "MultiplyWithRoot" null null))

(fn `UpdateNitro`
  (params (DeltaTime :type "Float (single-precision)"))
  (bind _damovements (`self.DaMovements`))
  (if (`self.HasNitro`)
    (set `self.Nitro` (- (`self.Nitro`) (* (`/Game/01_BP/04_DataAssets/BP_DA_TankMovements.NitroDrawRate` (`self.DaMovements`)) DeltaTime))))
  (if (`self.RechargingNitro`)
    (set `self.Nitro` (`KismetMathLibrary.FClamp` (+ (`self.Nitro`) (* (`/Game/01_BP/04_DataAssets/BP_DA_TankMovements.NitroRechargeRate` _damovements) DeltaTime)) 0.0 (`/Game/01_BP/04_DataAssets/BP_DA_TankMovements.NitroMax` _damovements)))))

(fn `UserConstructionScript`)