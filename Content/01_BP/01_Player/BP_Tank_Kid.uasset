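; Child tank Blueprint that animates left and right treads as instanced meshes along two splines.
; BeginPlay spaces the track instances evenly along each spline.
; Tick slides them by wrapped TrackTimeL/R, orienting them to the spline and dirtying render state only on the last index, with a debug print per link.
; Ground-alignment movement logic is disconnected, and the spline-mesh track builder PopulateSplineWithTracks is never called here.
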(event `self.ReceiveBeginPlay`
  (`parent.ReceiveBeginPlay`)
  ; Track Population setup (for INSTANCES)
  (`InstancedStaticMeshComponent.ClearInstances` (`self.Track`))
  (for _index (range (+ (- (* (`self.TrackNumber`) 2) 0) 1))
    (bind _returnvalue (<= _index (- (`self.TrackNumber`) 1)))
    (bind (_returnvalue_location _returnvalue_rotation _returnvalue_scale) (`KismetMathLibrary.BreakTransform` (`SplineComponent.GetTransformAtTime` (select `bool` _returnvalue :`false` (`self.Spline_L`) :`true` (`self.Spline_R`)) (* (`KismetMathLibrary.SelectInt` _index (- _index (`self.TrackNumber`)) _returnvalue) (/ (`KismetMathLibrary.Conv_IntToDouble` 1) (`self.TrackNumber`))) "World" true true)))
    (`InstancedStaticMeshComponent.AddInstance` (`self.Track`) (`KismetMathLibrary.MakeTransform` _returnvalue_location _returnvalue_rotation _returnvalue_scale) true)))

(event `self.ReceiveTick`
  (params (DeltaSeconds :type "Float (single-precision)"))
  (bind _tracknumber (`self.TrackNumber`))
  (bind _returnvalue (- (* _tracknumber 2) 0))
  (`parent.ReceiveTick` DeltaSeconds)
  (for _index (range (+ _returnvalue 1))
    (bind _returnvalue_2 (< _index _tracknumber))
    (bind _returnvalue_3 (`KismetMathLibrary.SelectFloat` (mod (`self.TrackTimeL`) 1.0) (mod (`self.TrackTimeR`) 1.0) _returnvalue_2))
    (bind _returnvalue_4 (select `bool` (> _returnvalue_3 0.0) :`false` (- 1.0 (`KismetMathLibrary.Abs` _returnvalue_3)) :`true` _returnvalue_3))
    (`KismetSystemLibrary.PrintString` (`KismetStringLibrary.Conv_DoubleToString` _returnvalue_4) true true (struct :`G` 0.66 :`B` 1.0 :`A` 1.0) 0.0)
    (bind _returnvalue_5 (select `bool` _returnvalue_2 :`false` (`self.Spline_L`) :`true` (`self.Spline_R`)))
    (`InstancedStaticMeshComponent.UpdateInstanceTransform` (`self.Track`) _index (`KismetMathLibrary.MakeTransform` (.location (`SplineComponent.GetTransformAtTime` _returnvalue_5 (mod (+ (* (`KismetMathLibrary.SelectInt` _index (- _index (`self.TrackNumber`)) _returnvalue_2) (/ (`KismetMathLibrary.Conv_IntToDouble` 1) (`self.TrackNumber`))) _returnvalue_4) 1.0) "World" true false)) (`KismetMathLibrary.MakeRotFromXY` (`KismetMathLibrary.GetForwardVector` (.rotation (`SplineComponent.GetTransformAtTime` _returnvalue_5 (mod (+ (* (`KismetMathLibrary.SelectInt` _index (- _index (`self.TrackNumber`)) _returnvalue_2) (/ (`KismetMathLibrary.Conv_IntToDouble` 1) (`self.TrackNumber`))) _returnvalue_4) 1.0) "World" true false))) (* (`SceneComponent.GetRightVector` _returnvalue_5) -1.0))) true (== _index _returnvalue) false)))

(fn `PopulateSplineWithTracks`
  (params (Spline :type "SplineComponent Object Reference") (StaticMesh :type "StaticMeshComponent Object Reference"))
  (bind _staticmesh (`StaticMeshComponent.StaticMesh` StaticMesh))
  (bind _tracklenght (`self.TrackLenght`))
  (bind (_returnvalue_min _returnvalue_max) (break `Box` (`StaticMesh.GetBoundingBox` _staticmesh)))
  (bind _returnvalue_x (`KismetMathLibrary.BreakVector` (+ (`KismetMathLibrary.Vector_GetAbs` _returnvalue_min) (`KismetMathLibrary.Vector_GetAbs` _returnvalue_max))))
  (bind _output_get (set `self.TrackLenght` _returnvalue_x))
  (for _index (range (+ (`KismetMathLibrary.FTrunc` (/ (`SplineComponent.GetSplineLength` Spline) _output_get)) 1))
    (bind _returnvalue (`AddComponent|NODE_AddSplineMeshComponent-1` :`RelativeTransform` (`SceneComponent.K2_GetComponentToWorld` Spline)))
    (`SplineMeshComponent.SetForwardAxis` _returnvalue "X" true)
    (`StaticMeshComponent.SetStaticMesh` _returnvalue _staticmesh)
    (bind _returnvalue_2 (* _index _tracklenght))
    (bind _returnvalue_3 (* _tracklenght (+ _index 1)))
    (`SplineMeshComponent.SetStartAndEnd` _returnvalue (`SplineComponent.GetLocationAtDistanceAlongSpline` Spline _returnvalue_2 "Local") (`KismetMathLibrary.ClampVectorSize` (`SplineComponent.GetTangentAtDistanceAlongSpline` Spline _returnvalue_2 "Local") 0.0 (`self.TrackLenght`)) (`SplineComponent.GetLocationAtDistanceAlongSpline` Spline _returnvalue_3 "Local") (`KismetMathLibrary.ClampVectorSize` (`SplineComponent.GetTangentAtDistanceAlongSpline` Spline _returnvalue_3 "Local") 0.0 (`self.TrackLenght`)) true)))

(fn `UserConstructionScript`
  (`parent.UserConstructionScript`))