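; Destructible crate that breaks apart when a tank or tank projectile overlaps its CollsionDestruction component.
; The overlap spawns a temporary FS_MasterField at the other actor's location, with stronger strain but smaller scale for tanks than projectiles.
; It plays a break sound and triggers the field, removing it and the collision component shortly after.
; The crate destroys itself after a longer delay.
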(event `self.collsion destruction.OnComponentBeginOverlap`
  (params (OverlappedComponent :type "PrimitiveComponent Object Reference") (OtherActor :type "Actor Object Reference") (OtherComp :type "PrimitiveComponent Object Reference") (OtherBodyIndex :type Integer) (bFromSweep :type Boolean) (SweepResult :type "HitResult Structure (by ref)"))
  (bind _asbp_tank (cast `/Game/01_BP/01_Player/BP_Tank` OtherActor)
    (:`then`
      (set `self.NewVar` (`self.K2_GetActorLocation` _asbp_tank))
      (set `self.projectile` true)
      (set `self.Scale` (3.0 3.0 3.0)))
    (:`CastFailed`
      (bind _asbp_tank_projectile (cast `/Game/01_BP/01_Player/BP_TankProjectile` OtherActor))
      (set `self.NewVar` (`self.K2_GetActorLocation` _asbp_tank_projectile))
      (set `self.projectile` false)
      (set `self.Scale` (5.0 5.0 5.0))))
  (bind _returnvalue (`|SpawnActorFromClass` "/Engine/EditorResources/FieldNodes/FS_MasterField.FS_MasterField_C" (`KismetMathLibrary.MakeTransform` (`self.NewVar`) (struct) (`self.Scale`)) "Undefined" "MultiplyWithRoot" null null))
  (`GameplayStatics.PlaySoundAtLocation` "/Game/08_Sfx/MetaSounds/MS_Deco_Breaks.MS_Deco_Breaks" (`self.K2_GetActorLocation`) (struct) 1.0 1.0 0.0 null null null null)
  (if (`self.projectile`)
    (set `/Engine/EditorResources/FieldNodes/FS_MasterField.Strain Magnitude` 1000000000.0 _returnvalue)
    (else
      (set `/Engine/EditorResources/FieldNodes/FS_MasterField.Strain Magnitude` 1000000.0 _returnvalue)))
  (set `/Engine/EditorResources/FieldNodes/FS_MasterField.ActivationType` "NewEnumerator4" _returnvalue)
  (`/Engine/EditorResources/FieldNodes/FS_MasterField.CE_Trigger` _returnvalue)
  (`KismetSystemLibrary.Delay` 0.2)
  (`self.K2_DestroyActor` _returnvalue)
  (`ActorComponent.K2_DestroyComponent` (`self.collsion destruction`))
  (`KismetSystemLibrary.Delay` 20.0)
  (`self.K2_DestroyActor`))

(fn `UserConstructionScript`)