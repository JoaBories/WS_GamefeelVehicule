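; BP_Tree_Destructible_2 is a destructible tree actor that breaks when a BP_Tank overlaps its CollsionDestruction component.
; The overlap spawns a temporary, scaled-up FS_MasterField at the tank's location with very high strain, then triggers it to apply the destruction force.
; The field is destroyed after a brief delay, and the tree actor removes itself some seconds later.
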(event `self.collsion destruction.OnComponentBeginOverlap`
  (params (OverlappedComponent :type "PrimitiveComponent Object Reference") (OtherActor :type "Actor Object Reference") (OtherComp :type "PrimitiveComponent Object Reference") (OtherBodyIndex :type Integer) (bFromSweep :type Boolean) (SweepResult :type "HitResult Structure (by ref)"))
  (bind _asbp_tank (cast `/Game/01_BP/01_Player/BP_Tank` OtherActor))
  (bind _returnvalue (`|SpawnActorFromClass` "/Engine/EditorResources/FieldNodes/FS_MasterField.FS_MasterField_C" (`KismetMathLibrary.MakeTransform` (`self.K2_GetActorLocation` _asbp_tank) (struct) (3.0 3.0 3.0)) "Undefined" "MultiplyWithRoot" null null))
  (set `/Engine/EditorResources/FieldNodes/FS_MasterField.Strain Magnitude` 1000000.0 _returnvalue)
  (set `/Engine/EditorResources/FieldNodes/FS_MasterField.ActivationType` "NewEnumerator4" _returnvalue)
  (`/Engine/EditorResources/FieldNodes/FS_MasterField.CE_Trigger` _returnvalue)
  (`KismetSystemLibrary.Delay` 0.2)
  (`self.K2_DestroyActor` _returnvalue)
  (`KismetSystemLibrary.Delay` 20.0)
  (`self.K2_DestroyActor`))

(fn `UserConstructionScript`)