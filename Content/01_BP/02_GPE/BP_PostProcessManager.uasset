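; BP_PostProcessManager drives the blend weights of two post-process effects, Explosion and Boost.
; Set events raise each effect's intensity to the requested value only if it exceeds the current one.
; Tick decays both intensities toward zero at separate speeds, clamped between 0 and 1, then applies them as blend weights.
; A debug event toggles the decay to freeze or resume the fade, while weights keep being applied every frame.
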(event `DEBUG_PlayPause`
  (set `self.NeedUpdate` (not (`self.NeedUpdate`))))

(event `self.ReceiveTick`
  (params (DeltaSeconds :type "Float (single-precision)"))
  (`|ExecutionSequence`
    (:`then_0`
      (if (`self.NeedUpdate`)
        (set `self.Expl` (`KismetMathLibrary.FClamp` (- (`self.Expl`) (* DeltaSeconds (`self.ExplDownSpeed`)))))
        (set `self.Turbo` (`KismetMathLibrary.FClamp` (- (`self.Turbo`) (* DeltaSeconds (`self.TurboDownSpeed`)))))))
    (:`then_1`
      (`self.Set Post Processes`))))

(event `Set Boost Effect`
  (params (`Wanted Value` :type "Float (double-precision)"))
  (set `self.Turbo` (`KismetMathLibrary.FMax` `Wanted Value` (`self.Turbo`))))

(event `Set Explosion Effect`
  (params (`Wanted Value` :type "Float (double-precision)"))
  (set `self.Expl` (`KismetMathLibrary.FMax` `Wanted Value` (`self.Expl`))))

(event `Set Post Processes`
  (set `PostProcessComponent.BlendWeight` (`self.Expl`) (`self.Explosion`))
  (set `PostProcessComponent.BlendWeight` (`self.Turbo`) (`self.Boost`)))

(fn `UserConstructionScript`)