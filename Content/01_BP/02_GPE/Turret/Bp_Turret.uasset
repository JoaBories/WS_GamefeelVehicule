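; Enemy turret that tracks and shoots the player within an activation distance, tuned by a BPDA_Turret data asset.
; Tick toggles activation by distance, smoothly turns the turret toward the player, spins the barrel, rotates the health bar and draws a debug aim line.
; After an activation delay, a re-arming timer spawns BP_TurretBullet with sound and VFX at the data asset's fire rate.
; Defeat deactivates and hides the turret.
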(event `DEBUG_ShowDistance`
  (`SceneComponent.SetWorldScale3D` (`self.DEBUG_DistanceSphere`) (* (`self.DEBUG_ActivationDist`) (0.01 0.01 0.01) 0.5)))

(event `self.ReceiveBeginPlay`
  (`parent.ReceiveBeginPlay`)
  (bind _asbpda_turret (cast `/Game/01_BP/02_GPE/Turret/BPDA_Turret` (`self.DataAsset`))
    (:`then`
      (set `self.TurretDA` _asbpda_turret)
      (`self.Activate`))
    (:`CastFailed`
      (`KismetSystemLibrary.PrintString` (`KismetStringLibrary.Concat_StrStr` "/!\\ ERROR: PLEASE PUT A TURRET DATA ASSET IN: " (`KismetSystemLibrary.GetDisplayName` self)) true true (struct :`R` 1.0 :`G` 0.032306 :`A` 1.0) 10.0))))

(event `self.ReceiveTick`
  (params (DeltaSeconds :type "Float (single-precision)"))
  (bind _mesh (`self.Mesh`))
  (bind _returnvalue (`SceneComponent.K2_GetComponentLocation` _mesh))
  (bind (_returnvalue_roll _returnvalue_pitch _returnvalue_yaw) (`KismetMathLibrary.BreakRotator` (`SceneComponent.K2_GetComponentRotation` (`self.TurretBoxCenter`))))
  (bind (_returnvalue_roll_2 _returnvalue_pitch_2 _returnvalue_yaw_2) (`KismetMathLibrary.BreakRotator` (`KismetMathLibrary.FindLookAtRotation` (`SceneComponent.K2_GetComponentLocation` (`self.TurretBoxCenter`)) (`self.K2_GetActorLocation` (`GameplayStatics.GetPlayerPawn` 0)))))
  (bind _returnvalue_2 (<= (`KismetMathLibrary.VSize` (- (`self.K2_GetActorLocation` (`GameplayStatics.GetPlayerPawn` 0)) (`self.K2_GetActorLocation`))) (`/Game/01_BP/02_GPE/Turret/BPDA_Turret.ActivationDistance` (`self.TurretDA`))))
  (bind _yaw (.yaw (`KismetMathLibrary.RLerp` (`KismetMathLibrary.MakeRotator` _returnvalue_roll _returnvalue_pitch _returnvalue_yaw) (`KismetMathLibrary.MakeRotator` _returnvalue_roll_2 _returnvalue_pitch_2 (- _returnvalue_yaw_2 90.0)) (* (`/Game/01_BP/02_GPE/Turret/BPDA_Turret.TurnRateAlpha` (`self.TurretDA`)) 0.01) true)))
  (if (not (`self.isDestroyed`))
    (`self.Rotate HealthBar`)
    (set `self.FireRateTimer` (+ DeltaSeconds (`self.FireRateTimer`)))
    (if (`self.Activated`)
      (if _returnvalue_2
        (`SceneComponent.K2_SetWorldRotation` (`self.TurretBoxCenter`) (`KismetMathLibrary.MakeRotator` (.roll (`KismetMathLibrary.RLerp` (`KismetMathLibrary.MakeRotator` _returnvalue_roll _returnvalue_pitch _returnvalue_yaw) (`KismetMathLibrary.MakeRotator` _returnvalue_roll_2 _returnvalue_pitch_2 (- _returnvalue_yaw_2 90.0)) (* (`/Game/01_BP/02_GPE/Turret/BPDA_Turret.TurnRateAlpha` (`self.TurretDA`)) 0.01) true)) (.pitch (`KismetMathLibrary.RLerp` (`KismetMathLibrary.MakeRotator` _returnvalue_roll _returnvalue_pitch _returnvalue_yaw) (`KismetMathLibrary.MakeRotator` _returnvalue_roll_2 _returnvalue_pitch_2 (- _returnvalue_yaw_2 90.0)) (* (`/Game/01_BP/02_GPE/Turret/BPDA_Turret.TurnRateAlpha` (`self.TurretDA`)) 0.01) true)) _yaw) false false)
        (`SceneComponent.K2_SetWorldRotation` (`self.Mesh`) (`KismetMathLibrary.MakeRotator` 0.0 0.0 _yaw) false false)
        (`KismetSystemLibrary.DrawDebugLine` _returnvalue (+ _returnvalue (* (`SceneComponent.GetForwardVector` _mesh) 5000.0)) (struct :`R` 1.0 :`B` 0.762551 :`A` 1.0) 0.0 2.0)
        (`SceneComponent.K2_AddLocalRotation` (`self.RotationCenter`) (`KismetMathLibrary.MakeRotator` 0.0 (* (`GameplayStatics.GetWorldDeltaSeconds`) (`/Game/01_BP/02_GPE/Turret/BPDA_Turret.BarilRotationRate` (`self.TurretDA`)))) false false)
        (else
          (`self.Deactivate`)))
      (elif _returnvalue_2
        (`self.Activate`)))))

(event `self.OnDefeated`
  (`self.Deactivate`)
  (`SceneComponent.SetVisibility` (`self.Turret`) false true))

(event `Activate`
  (set `self.Activated` true)
  (`KismetSystemLibrary.Delay` (`/Game/01_BP/02_GPE/Turret/BPDA_Turret.ActivationDelay` (`self.TurretDA`)))
  (`KismetSystemLibrary.K2_SetTimerDelegate` (delegate `Shoot`) (`/Game/01_BP/02_GPE/Turret/BPDA_Turret.FireRate` (`self.TurretDA`))))

(event `Deactivate`
  (set `self.Activated` false))

(event `Shoot`
  (bind _turretda (`self.TurretDA`))
  (bind _turretboxcenter (`self.TurretBoxCenter`))
  (bind _endbaril (`self.EndBaril`))
  (bind (_returnvalue_roll _returnvalue_pitch _returnvalue_yaw) (`KismetMathLibrary.BreakRotator` (`SceneComponent.K2_GetComponentRotation` _turretboxcenter)))
  (if (`self.isDestroyed`)
    _
    (elif (`self.Activated`)
      (`KismetSystemLibrary.K2_SetTimerDelegate` (delegate `Shoot`) (`/Game/01_BP/02_GPE/Turret/BPDA_Turret.FireRate` (`self.TurretDA`)) false true)
      (bind _returnvalue (`|SpawnActorFromClass` "/Game/01_BP/02_GPE/Turret/BP_TurretBullet.BP_TurretBullet_C" (`KismetMathLibrary.MakeTransform` (`SceneComponent.K2_GetComponentLocation` _turretboxcenter) (`KismetMathLibrary.MakeRotator` _returnvalue_roll _returnvalue_pitch (+ _returnvalue_yaw 90.0))) "Undefined" "MultiplyWithRoot" null null))
      (`/Game/01_BP/02_GPE/Turret/BP_TurretBullet.Start` _returnvalue (`/Game/01_BP/02_GPE/Turret/BPDA_Turret.Speed` _turretda) (`/Game/01_BP/02_GPE/Turret/BPDA_Turret.Damage` _turretda) (`/Game/01_BP/02_GPE/Turret/BPDA_Turret.HitVFX` _turretda) null)
      (`GameplayStatics.SpawnSoundAtLocation` (`/Game/01_BP/02_GPE/Turret/BPDA_Turret.ShootSFX` (`self.TurretDA`)) (`self.K2_GetActorLocation`) (struct) 1.0 1.0 0.0 null null)
      (`NiagaraFunctionLibrary.SpawnSystemAtLocation` (`/Game/01_BP/02_GPE/Turret/BPDA_Turret.ShootVFX` (`self.TurretDA`)) (`SceneComponent.K2_GetComponentLocation` _endbaril) (`SceneComponent.K2_GetComponentRotation` _endbaril)))))

(fn `UserConstructionScript`
  (`parent.UserConstructionScript`))