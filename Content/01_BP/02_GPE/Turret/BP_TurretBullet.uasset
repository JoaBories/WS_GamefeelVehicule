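; Turret projectile that, once started, flies forward at a given speed and deals turret damage to what it hits, ignoring actors tagged Enemy.
; Each Tick line-traces from its last position to the current one to detect hits along its path.
; On impact it spawns the supplied VFX and sound, sends an explosion effect scaled by player distance to BP_PostProcessManager, then destroys itself.
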(event `Start`
  (params (StartingSpeed :type "Float (double-precision)") (Damages :type "Float (double-precision)") (HitVFX :type "NiagaraSystem Object Reference") (HitSFX :type "MetaSoundSource Object Reference") (PPDistance :type "Float (double-precision)") (PPValue :type "Float (double-precision)"))
  (bind _projectilemovement (`self.ProjectileMovement`))
  (set `MovementComponent.Velocity` (* StartingSpeed (`self.GetActorForwardVector`)) _projectilemovement)
  (set `self.Damages` Damages)
  (`ActorComponent.Activate` _projectilemovement false)
  (set `self.HitVFX` HitVFX)
  (set `self.Hit SFX` HitSFX)
  (set `self.PPDistance` PPDistance)
  (set `self.PPValue` PPValue)
  (set `self.Lastposition` (`self.K2_GetActorLocation`)))

(event `self.ReceiveTick`
  (params (DeltaSeconds :type "Float (single-precision)"))
  (bind _returnvalue (`self.K2_GetActorLocation`))
  (bind (_outhit _returnvalue_2) (`KismetSystemLibrary.LineTraceSingleForObjects` :`Start` (`self.Lastposition`) :`End` (`self.K2_GetActorLocation`) :`ObjectTypes` (`|MakeArray` "ObjectTypeQuery1" "ObjectTypeQuery2" "ObjectTypeQuery3" :!type "EObjectTypeQuery Enum") :`DrawTime` 0.1))
  (if _returnvalue_2
    (bind (_bblockinghit _binitialoverlap _time _distance _location _impactpoint _normal _impactnormal _physmat _hitactor) (`GameplayStatics.BreakHitResult` _outhit))
    (`/Engine/EditorBlueprintResources/StandardMacros.IsValid` _hitactor
      (:`Is Valid`
        (if (`KismetArrayLibrary.Array_Contains` (`Actor.Tags` _hitactor) "Enemy")
          (set `self.Lastposition` (`self.K2_GetActorLocation`) :!label _label)
          (else
            (`GameplayStatics.ApplyDamage` _hitactor (`self.Damages`) null null "/Game/01_BP/06_DamageTypes/DT_Turret.DT_Turret_C")
            (`NiagaraFunctionLibrary.SpawnSystemAtLocation` (`self.HitVFX`) _returnvalue :!label _label_2)
            (`GameplayStatics.SpawnSoundAtLocation` (`self.Hit SFX`) _returnvalue (struct) 1.0 1.0 0.0 null null)
            (bind _returnvalue_3 (`GameplayStatics.GetActorOfClass` "/Game/01_BP/02_GPE/BP_PostProcessManager.BP_PostProcessManager_C"))
            (`/Engine/EditorBlueprintResources/StandardMacros.IsValid` _returnvalue_3
              (:`Is Valid`
                (`/Game/01_BP/02_GPE/BP_PostProcessManager.Set Explosion Effect` _returnvalue_3 (* (- 1.0 (/ (`KismetMathLibrary.Vector_Distance` (`self.K2_GetActorLocation` (`GameplayStatics.GetPlayerPawn` 0)) (`self.K2_GetActorLocation`)) (`self.PPDistance`))) (`self.PPValue`))))
              (:`Is Not Valid`
                (`KismetSystemLibrary.PrintString` "ADD POST PROCESS MANAGER" true true (struct :`R` 1.0 :`B` 0.018815 :`A` 1.0) 10.0)))
            (`self.K2_DestroyActor`))))
      (:`Is Not Valid`
        (goto _label_2)))
    (else
      (goto _label))))

(fn `UserConstructionScript`)