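; Parent Blueprint for destroyable objects that take damage and break, optionally dropping a health pickup.
; Life starts at the data asset's MaxLife and drops on AnyDamage, printing a debug hit message each time.
; At zero, a DoOnce flags it destroyed, plays the asset's VFX, swaps to the destroyed mesh, spawns any pickup, then calls OnDefeated, an empty event here.
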(event `self.ReceiveBeginPlay`
  (set `self.CurrentLife` (`/Game/01_BP/02_GPE/Destroyable_Parent/BPDA_DestroyableObject.MaxLife` (`self.DataAsset`))))

(event `self.ReceiveAnyDamage`
  (params (Damage :type "Float (single-precision)") (DamageType :type "DamageType Object Reference") (InstigatedBy :type "Controller Object Reference") (DamageCauser :type "Actor Object Reference"))
  (`KismetSystemLibrary.PrintString` (`KismetStringLibrary.Concat_StrStr` "HIT - " (`KismetSystemLibrary.GetDisplayName` self)) true false (struct :`R` 1.0 :`G` 0.103877 :`A` 1.0))
  (bind _output_get (set `self.CurrentLife` (- (`self.CurrentLife`) Damage)))
  (if (<= _output_get 0.0)
    (`/Engine/EditorBlueprintResources/StandardMacros.DoOnce` false
      (:`Completed`
        (set `self.isDestroyed` true)
        (`self.DestroyedFeedbacks`)
        (`self.OnDefeated`)))))

(event `DestroyedFeedbacks`
  (`NiagaraFunctionLibrary.SpawnSystemAttached` (`/Game/01_BP/02_GPE/Destroyable_Parent/BPDA_DestroyableObject.DestroyedVFX` (`self.DataAsset`)) (`self.Mesh`) "None" (0.0 0.0 0.0) (struct) "KeepRelativeOffset" true)
  (`StaticMeshComponent.SetStaticMesh` (`self.Mesh`) (`/Game/01_BP/02_GPE/Destroyable_Parent/BPDA_DestroyableObject.DestroyedMesh` (`self.DataAsset`)))
  (if (`self.DropHealthWhenDead`)
    (`|SpawnActorFromClass` "/Game/01_BP/02_GPE/HealthPickup/BP_HealthPickup.BP_HealthPickup_C" (`KismetMathLibrary.MakeTransform` (`self.K2_GetActorLocation`)) "Undefined" "MultiplyWithRoot" null null)))

(event `OnDefeated`)

(fn `UserConstructionScript`)