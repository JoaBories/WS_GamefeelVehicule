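; Health pickup actor that heals the player on contact, then destroys itself.
; Tick accumulates time to bob the actor with a per-frame sine offset and spin it around the vertical axis.
; Overlap by player pawn 0 on the Collision component applies negative damage as healing and spawns a VFX at the pickup's location.
; A data asset supplies the heal amount and effect.
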(event `self.ReceiveTick`
  (params (DeltaSeconds :type "Float (single-precision)"))
  (bind _output_get (set `self.Time` (+ DeltaSeconds (`self.Time`))))
  (`self.K2_AddActorWorldOffset` (`KismetMathLibrary.MakeVector` 0.0 0.0 (* (`KismetMathLibrary.Sin` _output_get) 0.05)))
  (`self.K2_SetActorRotation` (`KismetMathLibrary.MakeRotator` 0.0 0.0 (* _output_get 20.0))))

(event `self.Collision.OnComponentBeginOverlap`
  (params (OverlappedComponent :type "PrimitiveComponent Object Reference") (OtherActor :type "Actor Object Reference") (OtherComp :type "PrimitiveComponent Object Reference") (OtherBodyIndex :type Integer) (bFromSweep :type Boolean) (SweepResult :type "HitResult Structure (by ref)"))
  (if (== OtherActor (`GameplayStatics.GetPlayerPawn` 0))
    (`GameplayStatics.ApplyDamage` OtherActor (* (`/Game/01_BP/02_GPE/HealthPickup/BPDA_HealthPickup.AddedHealth` (`self.DataAsset`)) -1.0))
    (`NiagaraFunctionLibrary.SpawnSystemAtLocation` (`/Game/01_BP/02_GPE/HealthPickup/BPDA_HealthPickup.HealthVFX` (`self.DataAsset`)) (`self.K2_GetActorLocation`))
    (`self.K2_DestroyActor`)))

(fn `UserConstructionScript`)