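; Destroyable gameplay object with a life pool, configured by a data asset that supplies its max life and destroyed mesh.
; Any damage lowers current life; at zero or below it swaps to the destroyed mesh, then calls OnDefeated, an empty event here.
; Nothing guards against repeat defeat, so further hits trigger both again.
; A debug event applies a set damage amount to itself.
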(event `self.ReceiveBeginPlay`
  (set `self.CurrentLife` (`/Game/01_BP/02_GPE/Shields/BPDA_DestroyableObject.MaxLife` (`self.DataAsset`))))

(event `self.ReceiveAnyDamage`
  (params (Damage :type "Float (single-precision)") (DamageType :type "DamageType Object Reference") (InstigatedBy :type "Controller Object Reference") (DamageCauser :type "Actor Object Reference"))
  (bind _output_get (set `self.CurrentLife` (- (`self.CurrentLife`) Damage)))
  (if (<= _output_get 0.0)
    (`self.DestroyedFeedbacks`)
    (`self.OnDefeated`)))

(event `DEBUG_Damage`
  (`GameplayStatics.ApplyDamage` self (`self.DEBUG_TakeDamage`)))

(event `DestroyedFeedbacks`
  (`StaticMeshComponent.SetStaticMesh` (`self.Mesh`) (`/Game/01_BP/02_GPE/Shields/BPDA_DestroyableObject.DestroyedMesh` (`self.DataAsset`))))

(event `OnDefeated`)

(fn `UserConstructionScript`)