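; Shield generator gameplay actor that switches its Shield on and off and shuts it down when the generator is defeated.
; ActivateShield turns the Shield on only if the generator is not destroyed and the Shield is not already active.
; OnDefeated deactivates the Shield and turns placeholder text into a red "Ouch.." message.
; Debug events expose activation through the same checks and direct deactivation.
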(event `self.OnDefeated`
  (bind _placeholder (`self.Placeholder`))
  (`/Game/01_BP/02_GPE/Shields/BP_Shield.Deactivate` (`self.Shield`))
  (`TextRenderComponent.K2_SetText` _placeholder "Ouch..")
  (`TextRenderComponent.SetTextRenderColor` _placeholder (make `Color` 0 0 255 255)))

(event `DEBUG_ActivateShield`
  (`self.Activate Shield`))

(event `DEBUG_DeactivateShield`
  (`/Game/01_BP/02_GPE/Shields/BP_Shield.Deactivate` (`self.Shield`)))

(event `Activate Shield`
  (if (`self.isDestroyed`)
    _
    (elif (not (`/Game/01_BP/02_GPE/Shields/BP_Shield.isActivated` (`self.Shield`)))
      (`/Game/01_BP/02_GPE/Shields/BP_Shield.Activate` (`self.Shield`)))))

(fn `UserConstructionScript`
  (`parent.UserConstructionScript`))