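; BP_Shield is a toggleable shield that destroys tank projectiles that touch it.
; Activate and Deactivate switch the Sphere component's visibility and collision between query-only and none, and track the state in IsActivated.
; StartActivated picks the initial state on BeginPlay.
; The sphere's begin-overlap event destroys only actors whose class is exactly BP_TankProjectile.
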(event `self.ReceiveBeginPlay`
  (if (`self.StartActivated`)
    (`self.Activate`)
    (else
      (`self.Deactivate`))))

(event `Activate`
  (bind _sphere (`self.Sphere`))
  (`SceneComponent.SetVisibility` _sphere true false)
  (`PrimitiveComponent.SetCollisionEnabled` _sphere "QueryOnly")
  (set `self.isActivated` true))

(event `Deactivate`
  (bind _sphere (`self.Sphere`))
  (`SceneComponent.SetVisibility` _sphere false false)
  (`PrimitiveComponent.SetCollisionEnabled` _sphere "NoCollision")
  (set `self.isActivated` false))

(event `self.Sphere.OnComponentBeginOverlap`
  (params (OverlappedComponent :type "PrimitiveComponent Object Reference") (OtherActor :type "Actor Object Reference") (OtherComp :type "PrimitiveComponent Object Reference") (OtherBodyIndex :type Integer) (bFromSweep :type Boolean) (SweepResult :type "HitResult Structure (by ref)"))
  (if (== (`GameplayStatics.GetObjectClass` OtherActor) "/Game/01_BP/01_Player/BP_TankProjectile.BP_TankProjectile_C")
    (`self.K2_DestroyActor` OtherActor)))

(fn `UserConstructionScript`)