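; BP_BombShell is a mortar projectile that flies in an arc to a Target actor and explodes on arrival.
; Start supplies the flight and blast settings; Tick lerps toward the Target's current location, adds a sine height offset scaled by the square root of MaxHeight, and orients along the path.
; At the end it plays VFX and sound, damages overlapped actors not tagged Enemy within half of Radius, then destroys the Target and itself.
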(event `self.ReceiveBeginPlay`
  (bind _returnvalue (`self.K2_GetActorLocation`))
  (set `self.StartLocation` _returnvalue)
  (set `self.LastLocation` _returnvalue))

(event `Start`
  (params (Target :type "/Game/01_BP/02_GPE/Mortar/BP_Target Object Reference") (Timer :type "Float (double-precision)") (MaxHeight :type "Float (double-precision)") (Damages :type "Float (double-precision)") (ExplodeSFX :type "MetaSoundSource Object Reference") (ExplodeVFX :type "NiagaraSystem Object Reference") (Radius :type "Float (double-precision)"))
  (set `self.Target` Target)
  (set `self.Timer` Timer)
  (set `self.Max Height` (`KismetMathLibrary.Sqrt` MaxHeight))
  (set `self.Damages` Damages)
  (set `self.Explode SFX` ExplodeSFX)
  (set `self.Explode VFX` ExplodeVFX)
  (set `self.Radius` Radius))

(event `self.ReceiveTick`
  (params (DeltaSeconds :type "Float (single-precision)"))
  (bind _returnvalue (`self.K2_GetActorLocation`))
  (bind _returnvalue_2 (/ (`self.CurrentTimer`) (`self.Timer`)))
  (bind (_returnvalue_x _returnvalue_y _returnvalue_z) (`KismetMathLibrary.BreakVector` (`KismetMathLibrary.VLerp` (`self.StartLocation`) (`self.K2_GetActorLocation` (`self.Target`)) _returnvalue_2)))
  (set `self.CurrentTimer` (+ DeltaSeconds (`self.CurrentTimer`)))
  (`self.K2_SetActorLocation` (`KismetMathLibrary.MakeVector` _returnvalue_x _returnvalue_y (+ _returnvalue_z (* (`KismetMathLibrary.Sin` (`KismetMathLibrary.MultiplyByPi` _returnvalue_2)) (`self.Max Height`)))))
  (`self.K2_SetActorRotation` (`KismetMathLibrary.FindLookAtRotation` (`self.K2_GetActorLocation`) (`self.LastLocation`)))
  (set `self.LastLocation` (`self.K2_GetActorLocation`))
  (if (>= _returnvalue_2 0.999)
    (`NiagaraFunctionLibrary.SpawnSystemAtLocation` (`self.Explode VFX`) _returnvalue)
    (`GameplayStatics.SpawnSoundAtLocation` (`self.Explode SFX`) _returnvalue (struct) 1.0 1.0 0.0 null null)
    (bind _outactors (`KismetSystemLibrary.SphereOverlapActors` (`self.K2_GetActorLocation`) (* (`self.Radius`) 0.5) (`|MakeArray` "ObjectTypeQuery2" "ObjectTypeQuery3" :!type "EObjectTypeQuery Enum")))
    (for _array_element _outactors
      (if (not (`KismetArrayLibrary.Array_Contains` (`Actor.Tags` _array_element) "Enemy"))
        (`GameplayStatics.ApplyDamage` _array_element (`self.Damages`) null null "/Game/01_BP/06_DamageTypes/DT_Mortar.DT_Mortar_C")))
    (`self.K2_DestroyActor` (`self.Target`))
    (`self.K2_DestroyActor`)))

(fn `UserConstructionScript`)