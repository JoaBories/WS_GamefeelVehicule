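; BP_Mortar is a destructible mortar turret that bombards the player while they are within activation range, tuned through a BPDA_Mortar data asset.
; Tick toggles activation by player distance and lerps the mesh toward the player, drawing a debug aim line.
; A self-rescheduling timer spawns a BP_Target at the player's position and launches a BP_BombShell toward it with fall time, added height and damage.
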(event `DEBUG_ShowDistance`
  (`SceneComponent.SetWorldScale3D` (`self.DEBUG_DistanceSphere`) (* (`self.DEBUG Activation Dist`) (0.01 0.01 0.01))))

(event `self.ReceiveBeginPlay`
  (`parent.ReceiveBeginPlay`)
  (bind _asbpda_mortar (cast `/Game/01_BP/02_GPE/Mortar/BPDA_Mortar` (`self.DataAsset`))
    (:`then`
      (set `self.MortarDA` _asbpda_mortar)
      (set `self.isActivated` true)
      (`KismetSystemLibrary.K2_SetTimerDelegate` (delegate `ShootTimer`) (`/Game/01_BP/02_GPE/Mortar/BPDA_Mortar.ShootDelay` (`self.MortarDA`)) false true))
    (:`CastFailed`
      (`KismetSystemLibrary.PrintString` (`KismetStringLibrary.Concat_StrStr` "/!\\ ERROR: PLEASE PUT A MORTAR DATA ASSET IN: " (`KismetSystemLibrary.GetDisplayName` self)) true true (struct :`R` 1.0 :`G` 0.032306 :`A` 1.0) 10.0))))

(event `self.ReceiveTick`
  (params (DeltaSeconds :type "Float (single-precision)"))
  (bind _mesh (`self.Mesh`))
  (bind _returnvalue (`SceneComponent.K2_GetComponentLocation` _mesh))
  (bind (_returnvalue_roll _returnvalue_pitch _returnvalue_yaw) (`KismetMathLibrary.BreakRotator` (`KismetMathLibrary.FindLookAtRotation` (`SceneComponent.K2_GetComponentLocation` (`self.Mesh`)) (`self.K2_GetActorLocation` (`GameplayStatics.GetPlayerPawn` 0)))))
  (bind _returnvalue_2 (<= (`KismetMathLibrary.VSize` (- (`self.K2_GetActorLocation` (`GameplayStatics.GetPlayerPawn` 0)) (`self.K2_GetActorLocation`))) (`/Game/01_BP/02_GPE/Mortar/BPDA_Mortar.ActivationDistance` (`self.MortarDA`))))
  (bind _yaw (.yaw (`KismetMathLibrary.RLerp` (`SceneComponent.K2_GetComponentRotation` (`self.Mesh`)) (`KismetMathLibrary.MakeRotator` _returnvalue_roll _returnvalue_pitch (- _returnvalue_yaw 90.0)) (* (`/Game/01_BP/02_GPE/Mortar/BPDA_Mortar.TurnRateAlpha` (`self.MortarDA`)) 0.01) true)))
  (if (not (`self.isDestroyed`))
    (`self.Rotate HealthBar`)
    (if (`self.isActivated`)
      (if _returnvalue_2
        (`SceneComponent.K2_SetWorldRotation` (`self.MortarBox`) (`KismetMathLibrary.MakeRotator` 0.0 (.pitch (`KismetMathLibrary.RLerp` (`SceneComponent.K2_GetComponentRotation` (`self.Mesh`)) (`KismetMathLibrary.MakeRotator` _returnvalue_roll _returnvalue_pitch (- _returnvalue_yaw 90.0)) (* (`/Game/01_BP/02_GPE/Mortar/BPDA_Mortar.TurnRateAlpha` (`self.MortarDA`)) 0.01) true)) _yaw) false false)
        (`SceneComponent.K2_SetWorldRotation` (`self.Mesh`) (`KismetMathLibrary.MakeRotator` 0.0 0.0 _yaw) false false)
        (`KismetSystemLibrary.DrawDebugLine` _returnvalue (+ _returnvalue (* (`SceneComponent.GetForwardVector` _mesh) 5000.0)) (struct :`R` 1.0 :`B` 0.762551 :`A` 1.0) 0.0 2.0)
        (else
          (`self.Deactivate`)))
      (elif _returnvalue_2
        (`self.Activate`)))))

(event `ShootTimer`
  (if (`self.isDestroyed`)
    _
    (elif (`self.isActivated`)
      (`KismetSystemLibrary.K2_SetTimerDelegate` (delegate `ShootTimer`) (`/Game/01_BP/02_GPE/Mortar/BPDA_Mortar.ShootDelay` (`self.MortarDA`)) false true)
      (`self.Shoot`))))

(event `Shoot`
  (bind _mortarda (`self.MortarDA`))
  (bind _returnvalue (`|SpawnActorFromClass` "/Game/01_BP/02_GPE/Mortar/BP_Target.BP_Target_C" (`KismetMathLibrary.MakeTransform` (`self.K2_GetActorLocation` (`GameplayStatics.GetPlayerPawn` 0)) (struct) (* (1.0 1.0 1.0) (`/Game/01_BP/02_GPE/Mortar/BPDA_Mortar.TargetRadius` (`self.MortarDA`)))) "Undefined" "MultiplyWithRoot" null null))
  (bind _returnvalue_2 (`|SpawnActorFromClass` "/Game/01_BP/02_GPE/Mortar/BP_BombShell.BP_BombShell_C" (`KismetMathLibrary.MakeTransform` (`self.K2_GetActorLocation`) (struct) (* (1.0 1.0 1.0) (`/Game/01_BP/02_GPE/Mortar/BPDA_Mortar.TargetRadius` (`self.MortarDA`)) 0.01)) "Undefined" "MultiplyWithRoot" null null))
  (`/Game/01_BP/02_GPE/Mortar/BP_BombShell.Start` _returnvalue_2 (`/Game/01_BP/02_GPE/Mortar/BPDA_Mortar.ShellFallTimer` _mortarda) _returnvalue (`/Game/01_BP/02_GPE/Mortar/BPDA_Mortar.AddedHeight` _mortarda) (`/Game/01_BP/02_GPE/Mortar/BPDA_Mortar.Damages` _mortarda)))

(event `Activate`
  (if (not (`self.isActivated`))
    (set `self.isActivated` true)
    (`KismetSystemLibrary.Delay` (`/Game/01_BP/02_GPE/Mortar/BPDA_Mortar.ActivationDelay` (`self.MortarDA`)))
    (`self.ShootTimer`)))

(event `Deactivate`
  (set `self.isActivated` false))

(fn `UserConstructionScript`
  (`parent.UserConstructionScript`))