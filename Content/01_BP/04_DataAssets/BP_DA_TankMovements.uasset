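; BP_DA_TankMovements is a tank movement data asset that exposes tuning values through helper functions.
; Acceleration and max velocity getters pick nitro values first, otherwise forward or backward values, using nested float selects.
; Rotate speed switches between nitro and normal values.
; A clamp helper keeps cannon pitch within the range stored in a vector's X and Y.
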(fn `ClampCanonPitch`
  (params (InPitch :type "Float (double-precision)"))
  (returns (OutPitch :type "Float (double-precision)"))
  (bind (_canonclamppitch_x _canonclamppitch_y) (`KismetMathLibrary.BreakVector2D` (`self.CanonClampPitch`)))
  (return (`KismetMathLibrary.FClamp` InPitch _canonclamppitch_x _canonclamppitch_y)))

(fn `GetAcceleration`
  (params (Nitro :type Boolean) (Forward :type Boolean))
  (returns (Acceleration :type "Float (double-precision)"))
  (return (`KismetMathLibrary.SelectFloat` (`self.NitroAcceleration`) (`KismetMathLibrary.SelectFloat` (`self.FowardAcceleration`) (`self.BackwardAcceleration`) Forward) Nitro)))

(fn `GetMaxVelocity`
  (params (Nitro :type Boolean) (Forward :type Boolean))
  (returns (MaxVelocity :type "Float (double-precision)"))
  (return (`KismetMathLibrary.SelectFloat` (`self.NitroMaxVelocity`) (`KismetMathLibrary.SelectFloat` (`self.ForwardMaxVelocity`) (`self.BackwardMaxVelocity`) Forward) Nitro)))

(fn `GetRotateSpeed`
  (params (Nitro :type Boolean))
  (returns (RotateSpeed :type "Float (double-precision)"))
  (return (`KismetMathLibrary.SelectFloat` (`self.NitroRotateSpeed`) (`self.RotateSpeed`) Nitro)))