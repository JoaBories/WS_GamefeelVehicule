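; Procedural cable actor that builds a main cable along its spline from the construction script, tiling non-colliding spline meshes by mesh length with clamped tangents.
; It then adds a random number of secondary splines, scaled to main length, linking points slightly below the main spline through randomly offset midpoints.
; These secondary splines get tiled with a second mesh.
; An alternative CableComponent-based branch exists but never runs.
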(event `generate spline mesh`
  (bind _lenght (`self.Lenght`))
  (bind _spline (`self.Spline`))
  (bind _spline_2 (`self.Spline`))
  (bind (_returnvalue_min _returnvalue_max) (break `Box` (`StaticMesh.GetBoundingBox` (`self.Mesh`))))
  (bind _returnvalue_x (`KismetMathLibrary.BreakVector` (+ (`KismetMathLibrary.Vector_GetAbs` _returnvalue_min) (`KismetMathLibrary.Vector_GetAbs` _returnvalue_max))))
  (bind _output_get (set `self.Lenght` _returnvalue_x))
  (bind _output_get_2 (set `self.last index` (`KismetMathLibrary.FTrunc` (/ (`SplineComponent.GetSplineLength` (`self.Spline`)) _output_get))))
  (for _index (range (+ _output_get_2 1))
    (bind _returnvalue (`AddComponent|NODE_AddSplineMeshComponent-0`))
    (`PrimitiveComponent.SetCastShadow` _returnvalue true)
    (`PrimitiveComponent.SetCollisionEnabled` _returnvalue "NoCollision")
    (`SplineMeshComponent.SetForwardAxis` _returnvalue "X" true)
    (`StaticMeshComponent.SetStaticMesh` _returnvalue (`self.Mesh`))
    (bind _returnvalue_2 (* _index _lenght))
    (bind _returnvalue_3 (* (+ _index 1) _lenght))
    (`SplineMeshComponent.SetStartAndEnd` _returnvalue (`SplineComponent.GetLocationAtDistanceAlongSpline` _spline _returnvalue_2 "Local") (`KismetMathLibrary.ClampVectorSize` (`SplineComponent.GetTangentAtDistanceAlongSpline` _spline _returnvalue_2 "Local") 0.0 (`self.Lenght`)) (`SplineComponent.GetLocationAtDistanceAlongSpline` _spline_2 _returnvalue_3 "Local") (`KismetMathLibrary.ClampVectorSize` (`SplineComponent.GetTangentAtDistanceAlongSpline` _spline_2 _returnvalue_3 "Local") 0.0 (`self.Lenght`)) true))
  (`self.add random cable mesh`))

(event `add random cable mesh`
  (bind _spline (`self.Spline`))
  (bind _returnvalue (`SplineComponent.GetSplineLength` (`self.Spline`)))
  (bind _output_get (set `self.distance float cables` (`KismetMathLibrary.RandomFloatInRange` 0.0 _returnvalue)))
  (for _ (range 1 (+ (`KismetMathLibrary.RandomIntegerInRange` 1 (`KismetMathLibrary.Round` (/ _returnvalue 500.0))) 1))
    (bind _returnvalue_2 (`AddComponent|NODE_AddSplineComponent-0`))
    (bind _returnvalue_3 (+ (`SplineComponent.GetLocationAtDistanceAlongSpline` _spline _output_get "Local") (0.0 0.0 -15.0)))
    (`SplineComponent.SetLocationAtSplinePoint` _returnvalue_2 0 _returnvalue_3 "Local" true)
    (bind _output_get_2 (set `self.end point temp` (+ (`SplineComponent.GetLocationAtDistanceAlongSpline` _spline (`KismetMathLibrary.RandomFloatInRange` 0.0 _returnvalue) "Local") (0.0 0.0 -15.0))))
    (`SplineComponent.AddSplinePoint` _returnvalue_2 _output_get_2 "Local" true)
    (`SplineComponent.SetLocationAtSplinePoint` _returnvalue_2 1 (+ (`KismetMathLibrary.VLerp` _returnvalue_3 _output_get_2 (`KismetMathLibrary.RandomFloatInRange` 0.4 0.6)) (`KismetMathLibrary.MakeVector` (`KismetMathLibrary.RandomFloatInRange` -200.0 200.0) (`KismetMathLibrary.RandomFloatInRange` -200.0 200.0))) "Local" true)
    (`self.generate smaller spline meshes` _returnvalue_2)))

(event `generate smaller spline meshes`
  (params (spline :type "SplineComponent Object Reference"))
  (bind _lenght (`self.Lenght`))
  (bind (_returnvalue_min _returnvalue_max) (break `Box` (`StaticMesh.GetBoundingBox` (`self.Mesh_smol`))))
  (bind _returnvalue_x (`KismetMathLibrary.BreakVector` (+ (`KismetMathLibrary.Vector_GetAbs` _returnvalue_min) (`KismetMathLibrary.Vector_GetAbs` _returnvalue_max))))
  (bind _output_get (set `self.Lenght` _returnvalue_x))
  (bind _output_get_2 (set `self.last index` (`KismetMathLibrary.FTrunc` (/ (`SplineComponent.GetSplineLength` spline) _output_get))))
  (for _index (range (+ _output_get_2 1))
    (bind _returnvalue (`AddComponent|NODE_AddSplineMeshComponent-2`))
    (`PrimitiveComponent.SetCastShadow` _returnvalue true)
    (`PrimitiveComponent.SetCollisionEnabled` _returnvalue "NoCollision")
    (`SplineMeshComponent.SetForwardAxis` _returnvalue "X" true)
    (`StaticMeshComponent.SetStaticMesh` _returnvalue (`self.Mesh_smol`))
    (bind _returnvalue_2 (* _index _lenght))
    (bind _returnvalue_3 (* (+ _index 1) _lenght))
    (`SplineMeshComponent.SetStartAndEnd` _returnvalue (`SplineComponent.GetLocationAtDistanceAlongSpline` spline _returnvalue_2 "Local") (`KismetMathLibrary.ClampVectorSize` (`SplineComponent.GetTangentAtDistanceAlongSpline` spline _returnvalue_2 "Local") 0.0 (`self.Lenght`)) (`SplineComponent.GetLocationAtDistanceAlongSpline` spline _returnvalue_3 "Local") (`KismetMathLibrary.ClampVectorSize` (`SplineComponent.GetTangentAtDistanceAlongSpline` spline _returnvalue_3 "Local") 0.0 (`self.Lenght`)) true)))

(fn `UserConstructionScript`
  (`self.generate spline mesh`))