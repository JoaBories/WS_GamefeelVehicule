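; Drone VFX Blueprint that stages a red drone's opening, laser firing and shutdown through Play and Stop events.
; PlayDroneVFX plays the opening animation, spawns anticipation Niagara, then shows the laser while chained timelines drive heat progress, then strength, in MPC_Drones.
; StopDroneVFX hides the laser, spawns an end effect, ramps heat progress down, and later plays the animation in reverse.
; Heat values live in a Material Parameter Collection, so they are global rather than per drone.
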(event `self.ReceiveBeginPlay`)

(event `Play Drone VFX`
  (bind _sk_drone_red (`self.SK_Drone_Red`))
  (bind _ns_laser_red (`self.NS_Laser_Red`))
  (`SkeletalMeshComponent.PlayAnimation` _sk_drone_red "/Game/07_Vfx/04_FX_old/05_Mesh/Drone/AN_Drone_Opening.AN_Drone_Opening" false)
  (`KismetSystemLibrary.Delay` 0.4)
  (`NiagaraFunctionLibrary.SpawnSystemAttached` "/Game/07_Vfx/04_FX_old/03_Niagara_Systems/Laser/NS_LaserAntisipation_Red.NS_LaserAntisipation_Red" _sk_drone_red "None" (0.0 0.0 0.0) (struct) "KeepRelativeOffset" true)
  (`KismetSystemLibrary.Delay` 2.5)
  (`SceneComponent.SetVisibility` _ns_laser_red true false)
  (`ActorComponent.Activate` _ns_laser_red true)
  (bind (_direction _heating_up) (`Timeline|HeatColor` :!via `PlayFromStart`)
    (:`Update`
      (`KismetMaterialLibrary.SetScalarParameterValue` "/Game/07_Vfx/04_FX_old/02_Material_Others/MPC_Drones.MPC_Drones" "Heated_Progress" _heating_up))
    (:`Finished`
      (bind (_direction_2 _heat_streagth) (`Timeline|Timeline`)
        (:`Update`
          (`KismetMaterialLibrary.SetScalarParameterValue` "/Game/07_Vfx/04_FX_old/02_Material_Others/MPC_Drones.MPC_Drones" "Heated_Strength" _heat_streagth))))))

(event `Stop Drone VFX`
  (bind _sk_drone_red (`self.SK_Drone_Red`))
  (`SceneComponent.SetVisibility` (`self.NS_Laser_Red`) false false)
  (`NiagaraFunctionLibrary.SpawnSystemAttached` "/Game/07_Vfx/04_FX_old/03_Niagara_Systems/Laser/NS_LaserEnd_Red.NS_LaserEnd_Red" (`self.SK_Drone_Red`) "None" (0.0 0.0 0.0) (struct) "KeepRelativeOffset")
  (`KismetSystemLibrary.Delay` 0.4)
  (`|ExecutionSequence`
    (:`then_0`
      (bind (_direction _heating_down) (`Timeline|HeatColorOff` :!via `PlayFromStart`)
        (:`Update`
          (`KismetMaterialLibrary.SetScalarParameterValue` "/Game/07_Vfx/04_FX_old/02_Material_Others/MPC_Drones.MPC_Drones" "Heated_Progress" _heating_down))))
    (:`then_1`
      (`KismetSystemLibrary.Delay` 2.5)
      (`SkeletalMeshComponent.SetPlayRate` _sk_drone_red -1.0)
      (`SkeletalMeshComponent.SetPosition` _sk_drone_red 1.0 true)
      (`SkeletalMeshComponent.Play` _sk_drone_red false))))

(fn `UserConstructionScript`)